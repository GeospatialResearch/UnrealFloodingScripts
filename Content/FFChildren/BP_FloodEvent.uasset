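; BP_FloodEvent manages a flood scenario level, handling its start time, on-screen clock, level transition and pause menu.
; On BeginPlay it plays a fade-in sequence and sets every flux modifier source's DepthTimeline to LevelStartFloodTime.
; A one-second looping timer shows one source's timeline position as hours:minutes:seconds in W_ClockWidget.
; F fades out and opens NextFloodLevel after a delay, while P pauses with W_PauseMenu.
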(event Custom|UpdateClock
  (bind _depth_timeline (Variables|Default|GetDepth%20Timeline))
  (bind _returnvalue (Components|Timeline|GetPlaybackPosition _depth_timeline))
  (bind (_remainder _returnvalue_2) (Math|Float|Division(WholeandRemainder) _returnvalue 3.6e+03))
  (bind (_remainder_2 _returnvalue_3) (Math|Float|Division(WholeandRemainder) _remainder 6e+01))
  (Variables|/Script/UMG.TextBlock|SetText (Variables|/Game/Widgets/W_ClockWidget.W_ClockWidget_C|GetClockDisplay (Variables|Default|GetClockWidget)) (Utilities|Text|ToText(String) (Utilities|String|Append (Utilities|String|ToString(Text) (Utilities|Text|ToText(Integer) _returnvalue_2 false true 2)) ":" (Utilities|String|ToString(Text) (Utilities|Text|ToText(Integer) _returnvalue_3 false true 2)) ":" (Utilities|String|ToString(Text) (Utilities|Text|ToText(Float) _remainder_2 "HalfToEven" false true 2 324 0 0))))))

(event Custom|ChangeLevel
  (params (LevelName :type Name))
  (if (== LevelName (Utilities|Name|MakeLiteralName "None"))
    (Development|PrintString "Level is not set")
    (else
      (bind _returnvalue (Sequencer|Player|CreateLevelSequencePlayer "/Game/Cinematics/LS_FadeOutToNextLevel.LS_FadeOutToNextLevel"))
      (Sequencer|Player|Play _returnvalue :!class /Script/MovieScene.MovieSceneSequencePlayer)
      (Utilities|FlowControl|Delay 3.0)
      (Game|OpenLevel(byName) LevelName))))

(event EventTick
  (params (DeltaSeconds :type Float%20%28single-precision%29)))

(event EventBeginPlay
  (bind _levelstartfloodtime (Variables|FloodEvent|GetLevelStartFloodTime))
  (Variables|Default|SetPlayerController (Game|GetPlayerController (Variables|/Script/Engine.Pawn|GetPlayerState (Game|Player|GetPlayerPawn 0))))
  (bind _returnvalue (Sequencer|Player|CreateLevelSequencePlayer "/Game/Cinematics/LS_FadeInToNewLevel.LS_FadeInToNewLevel"))
  (Sequencer|Player|Play _returnvalue :!class /Script/MovieScene.MovieSceneSequencePlayer)
  (Development|PrintString "Get Actor")
  (bind _returnvalue_2 (Actor|GetActorOfClass "/Game/FFChildren/BP_FluxModifierSourceActor_Child.BP_FluxModifierSourceActor_Child_C"))
  (Development|PrintString (Utilities|String|ToString(Boolean) (Utilities|IsValid _returnvalue_2)))
  (Variables|Default|SetDepth%20Timeline (Variables|/Game/FFChildren/BP_FluxModifierSourceActor_Child.BP_FluxModifierSourceActor_Child_C|GetDepthTimeline _returnvalue_2))
  (Development|PrintString (Utilities|String|Append (Utilities|String|ToString(Float) _levelstartfloodtime) " Seconds") true true "(R=0.000000,G=0.660000,B=1.000000,A=1.000000)" 5.0)
  (CallFunction|UpdateTime _levelstartfloodtime)
  (Utilities|Time|SetTimerbyEvent (delegate Custom|UpdateClock) 1.0 true)
  (bind _returnvalue_3 (UserInterface|CreateWidget "/Game/Widgets/W_ClockWidget.W_ClockWidget_C" (Variables|Default|GetPlayerController)))
  (bind _output_get (Variables|Default|SetClockWidget _returnvalue_3))
  (UserInterface|Viewport|AddtoViewport _output_get 0)
  (CallFunction|UpdateClock))

(event Input|KeyboardEvents|F
  (params (Key :type Key%20Structure))
  (bind _nextfloodlevel (Variables|FloodEvent|GetNextFloodLevel))
  (bind _returnvalue (Class|KismetSystemLibrary|ToSoftObjPath(SoftObjRef) _nextfloodlevel))
  (bind _pathstring (Utilities|BreakSoftObjectPath _returnvalue))
  (bind (_pathpart _filenamepart) (Utilities|String|Split _pathstring))
  (:Pressed
    (CallFunction|ChangeLevel (Utilities|String|StringToName (Utilities|String|Append _pathpart "/" _filenamepart)))))

(event Input|KeyboardEvents|P
  (params (Key :type Key%20Structure))
  (:Pressed
    (CallFunction|PauseGame)))

(fn ConstructionScript)

(fn UpdateTime
  (params (NewTime :type Float%20%28double-precision%29))
  (bind _outactors (Actor|GetAllActorsOfClass "/Game/FFChildren/BP_FluxModifierSourceActor_Child.BP_FluxModifierSourceActor_Child_C"))
  (for _array_element _outactors
    (Components|Timeline|SetPlaybackPosition (Variables|/Game/FFChildren/BP_FluxModifierSourceActor_Child.BP_FluxModifierSourceActor_Child_C|GetDepthTimeline _array_element) NewTime false true)))

(fn PauseGame
  (bind _playercontroller (Variables|Default|GetPlayerController))
  (Development|PrintString "Paused Game")
  (Utilities|IsValid (Variables|Default|GetPauseMenuReference)
    (:Is%20Valid
      _)
    (:Is%20Not%20Valid
      (bind _returnvalue (UserInterface|CreateWidget "/Game/Widgets/W_PauseMenu.W_PauseMenu_C"))
      (Variables|Default|SetPauseMenuReference _returnvalue)))
  (Variables|/Script/Engine.PlayerController|SetbShowMouseCursor _playercontroller true)
  (Input|SetInputModeUIOnly _playercontroller (Variables|Default|GetPauseMenuReference) "DoNotLock" false)
  (UserInterface|Viewport|AddtoViewport (Variables|Default|GetPauseMenuReference) 0)
  (Game|SetGamePaused true))
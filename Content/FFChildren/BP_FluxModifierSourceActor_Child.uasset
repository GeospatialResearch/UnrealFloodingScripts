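; Child Blueprint of a flux modifier source actor that animates the FluxModifierSource's Volume over time, apparently to vary depth.
; On BeginPlay it loads DepthTimeCurve into DepthTimeline, sets the length to the last key and plays it, writing the curve value to Volume on each update.
; A DisplayDepth debug event prints playback position and Volume, but its looping timer setup is disconnected.
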(event Custom|DisplayDepth
  (Development|PrintString (Utilities|String|Append (Utilities|String|ToString(Float) (Components|Timeline|GetPlaybackPosition (Variables|Default|GetDepthTimeline))) " - " (Utilities|String|ToString(Float) (Variables|/Game/FluidFlux/Simulation/Modifiers/Components/BP_FluxModifierSourceComponent.BP_FluxModifierSourceComponent_C|GetVolume (Variables|Default|GetFluxModifierSource))))))

(event EventBeginPlay
  (bind _depthtimeline (Variables|Default|GetDepthTimeline))
  (|CallParentFunction)
  (Class|TimelineComponent|SetFloatCurve _depthtimeline (Variables|Default|GetDepthTimeCurve) "DepthTimeCurve")
  (Class|TimelineComponent|SetTimelineLengthMode _depthtimeline "TL_LastKeyFrame")
  (bind _depthtimecurve (Timeline|DepthTimeline Play)
    (:Update
      (Variables|/Game/FluidFlux/Simulation/Modifiers/Components/BP_FluxModifierSourceComponent.BP_FluxModifierSourceComponent_C|SetVolume (Variables|Default|GetFluxModifierSource) _depthtimecurve))))

(event Collision|EventActorBeginOverlap
  (params (OtherActor :type Actor%20Object%20Reference)))

(event EventTick
  (params (DeltaSeconds :type Float%20%28single-precision%29))
  (|CallParentFunction DeltaSeconds))

(fn ConstructionScript
  (|CallParentFunction))